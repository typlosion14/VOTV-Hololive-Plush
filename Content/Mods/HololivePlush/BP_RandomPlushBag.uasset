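; Usable plush bag for the HololivePlush mod that spawns a random plush in front of the player and destroys itself.
; Right-hand use picks from PeluchesClasses, rerolling BP_SanaBeeg unless a weighted keep chance passes, then shows a hint and plays a sound.
; New plush names are added to the ModActor's obtained list; the holoPlushCollections achievement's progress is only logged, not changed here.
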(event `PrintToModLoader`
  (params (Message :type String)))

(event `/Game/main/interfaces/int_objects.playerHandUse_RMB`
  (params (player :type "/Game/main/mainPlayer Object Reference"))
  (bind _peluchesclasses (`self.PeluchesClasses`))
  (bind _achievements (`/Game/main/save_main.achievements` (`/Game/main/lib.getMainSave`)))
  (bind _output_get (set `self.PickedClass` (`|GetArrayItem` _peluchesclasses (`KismetMathLibrary.RandomIntegerInRange` 0 (- (`KismetArrayLibrary.Array_Length` _peluchesclasses) 1))) :!label _label))
  (if (and (== _output_get "/Game/Mods/HololivePlush/Sana/BP_SanaBeeg.BP_SanaBeeg_C") (not (`KismetMathLibrary.RandomBoolWithWeight` (`self.SanaBeegKeepChance`))))
    (goto _label)
    (else
      (bind _returnvalue (`|SpawnActorFromClass` _output_get (`KismetMathLibrary.Conv_VectorToTransform` (+ (`self.GetActorForwardVector` player) (`self.K2_GetActorLocation` player))) "Undefined" "OverrideRootScale" null "None" false false null))
      (bind _output (`self.getModActor`))
      (bind (_mesh _displayname) (break `/Game/main/structs/struct_prop` (`/Game/objects/prop.propData` _returnvalue)))
      (`/Game/main/mainGamemode.Add Hint from Gamemode` (`/Game/main/lib.getMainGamemode`) (`|FormatText` "You got {0}" _displayname) "NewEnumerator0" false)
      (`GameplayStatics.PlaySound2D` "/Game/audio/effects/mreopen_Cue.mreopen_Cue" 1.0 1.0 0.0 null null)
      (`self.K2_DestroyActor`)
      (bind _currentplushobtained (`/Game/Mods/HololivePlush/ModActor.currentPlushObtained` _output))
      (if (== (`KismetArrayLibrary.Array_Find` _currentplushobtained _displayname) -1)
        (`KismetArrayLibrary.Array_Add` _currentplushobtained _displayname)
        (for _array_element _achievements
          (bind (_name _image _displayname_2 _progresstarget _progress) (break `/Game/main/structs/struct_achievement` _array_element))
          (if (== _name "holoPlushCollections")
            (`self.PrintToModLoader` (`KismetTextLibrary.Conv_TextToString` (`|FormatText` "Improve Achievement {0} at {1} progress on {2}" _displayname_2 _progress _progresstarget)))))
        (else
          (for _array_element_2 _achievements
            (bind (_name_2 _image_2 _displayname_3 _progresstarget_2 _progress_2) (break `/Game/main/structs/struct_achievement` _array_element_2))
            (if (== _name_2 "holoPlushCollections")
              (`self.PrintToModLoader` (`KismetTextLibrary.Conv_TextToString` (`|FormatText` "Achievement {0} at {1} progress on {2}" _displayname_3 _progress_2 _progresstarget_2))))))))))

(fn `getModActor`
  (returns (Output :type "/Game/Mods/HololivePlush/ModActor Object Reference"))
  (bind _outactors (`GameplayStatics.GetAllActorsOfClass` "/Game/Mods/HololivePlush/ModActor.ModActor_C"))
  (bind _output (`|GetArrayItem` _outactors))
  (if (`KismetSystemLibrary.IsValid` _output)
    (return _output)))

(fn `UserConstructionScript`
  (`parent.UserConstructionScript`))