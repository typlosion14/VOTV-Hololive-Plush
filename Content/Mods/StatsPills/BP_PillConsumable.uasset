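; Consumable hunger pill actor for the StatsPills mod, used by right-clicking with it in the player's hand.
; Each use increments the hunger dose counter on the shared ModActor, found by class lookup, up to a cap of five.
; A successful use shows a count hint, plays an eating sound and destroys the pill; at the cap it only shows a warning hint.
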(event `PrintToModLoader`
  (params (Message :type String)))

(event `/Game/main/interfaces/int_objects.playerHandUse_RMB`
  (params (player :type "/Game/main/mainPlayer Object Reference"))
  (`self.PrintToModLoader` "Pill used")
  (bind _output (`self.getModActor`))
  (bind _currentdosesh (`/Game/Mods/StatsPills/ModActor.currentDosesH` _output))
  (if (< _currentdosesh 5)
    (bind _output_get (set `/Game/Mods/StatsPills/ModActor.currentDosesH` (`KismetMathLibrary.Clamp` (+ _currentdosesh 1) 0 5) _output))
    (`/Game/main/mainGamemode.Add Hint from Gamemode` (`/Game/main/lib.getMainGamemode`) (`|FormatText` "Hunger Pill took ({0}/5)" (`KismetTextLibrary.Conv_IntToText` _output_get)) "NewEnumerator0" false)
    (`GameplayStatics.PlaySound2D` "/Game/audio/ui/eat_soft_Cue.eat_soft_Cue" 1.0 1.0 0.0 null null)
    (`self.K2_DestroyActor`)
    (else
      (`/Game/main/mainGamemode.Add Hint from Gamemode` (`/Game/main/lib.getMainGamemode`) "Maximum number of pills taken" "NewEnumerator0" false))))

(fn `getModActor`
  (returns (Output :type "/Game/Mods/StatsPills/ModActor Object Reference"))
  (bind _outactors (`GameplayStatics.GetAllActorsOfClass` "/Game/Mods/StatsPills/ModActor.ModActor_C"))
  (bind _output (`|GetArrayItem` _outactors))
  (if (`KismetSystemLibrary.IsValid` _output)
    (return _output)))

(fn `UserConstructionScript`)